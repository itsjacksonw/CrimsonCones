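; Boss enemy character that chases the player once PawnSensing spots them and attacks in melee.
; FollowPlayer runs AI MoveTo; on arrival within attack range it locks movement, plays a punch animation, and damages Player-tagged actors in a delayed sphere overlap at the fist.
; It then restores walking and its Animation Blueprint.
; Incoming damage reduces Health, and at zero the boss is destroyed and prints a win message.
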(event `self.PawnSensing.OnSeePawn`
  (params (Pawn :type "Pawn Object Reference"))
  (set `self.isSeeingPlayer` true)
  (`self.FollowPlayer`))

(event `FollowPlayer`
  (bind _mesh (`self.Mesh`))
  (if (`self.isSeeingPlayer`)
    (`|AIMoveTo` self (0.0 0.0 0.0) (`GameplayStatics.GetPlayerCharacter` 0)
      (:`then`
        (if (`self.canAttack`)
          (if (<= (`KismetMathLibrary.Vector_Distance` (`self.K2_GetActorLocation`) (`self.K2_GetActorLocation` (`GameplayStatics.GetPlayerCharacter` 0))) (`self.Melee Attack Distance`))
            (set `self.canAttack` false)
            (`SkeletalMeshComponent.PlayAnimation` (`self.Mesh`) "/Game/ThirdPerson/Blueprints/Standing_Melee_Attack_Horizontal_1_.Standing_Melee_Attack_Horizontal_1_" false)
            (`CharacterMovementComponent.DisableMovement` (`self.CharacterMovement`))
            (`SkeletalMeshComponent.PlayAnimation` (`self.Mesh`) "/Game/ThirdPerson/Blueprints/Boss_Punch.Boss_Punch" false)
            (`KismetSystemLibrary.Delay` 0.75)
            (bind _outactors (`KismetSystemLibrary.SphereOverlapActors` (`SceneComponent.K2_GetComponentLocation` (`self.Punch`)) 50.0 (`self.Object Types`)))
            (for _array_element _outactors
              (if (`self.ActorHasTag` _array_element "Player")
                (`GameplayStatics.ApplyDamage` _array_element 5.0)))
            (`KismetSystemLibrary.Delay` 0.75)
            (`CharacterMovementComponent.SetMovementMode` (`self.CharacterMovement`) "MOVE_Walking" 0)
            (`SkeletalMeshComponent.SetAnimationMode` _mesh "AnimationBlueprint")
            (`SkeletalMeshComponent.SetAnimInstanceClass` _mesh "/Game/Animations/AnimBlueprintBoss.AnimBlueprintBoss_C")
            (set `self.canAttack` true)))))))

(event `self.ReceiveAnyDamage`
  (params (Damage :type "Float (single-precision)") (DamageType :type "DamageType Object Reference") (InstigatedBy :type "Controller Object Reference") (DamageCauser :type "Actor Object Reference"))
  (set `self.Health` (- (`self.Health`) Damage))
  (`KismetSystemLibrary.PrintString` (`KismetStringLibrary.Conv_DoubleToString` (`self.Health`)))
  (if (<= (`self.Health`) 0.0)
    (`self.K2_DestroyActor`)
    (`KismetSystemLibrary.PrintString` "U has win")))

(fn `UserConstructionScript`)