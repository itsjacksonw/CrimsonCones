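; Boss enemy that chases the player on sight and alternates randomly between a close punch and a jumping slam.
; Pawn sensing triggers an AI move, then range-checked attacks pause movement, play animations and damage Player-tagged actors via sphere overlaps.
; The slam also relocates the boss toward the player afterward.
; Incoming damage drains health until destruction and spawns a ground-traced healing blood pickup on every third hit, starting with the first.
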(event `self.PawnSensing.OnSeePawn`
  (params (Pawn :type "Pawn Object Reference"))
  (set `self.isSeeingPlayer` true)
  (`self.FollowPlayer`))

(event `FollowPlayer`
  (bind _returnvalue (`self.K2_GetActorLocation`))
  (bind _mesh (`self.Mesh`))
  (bind _mesh_2 (`self.Mesh`))
  (if (`self.isSeeingPlayer`)
    (if (`self.canAttack`)
      (`|AIMoveTo` self (0.0 0.0 0.0) (`GameplayStatics.GetPlayerCharacter` 0)
        (:`then`
          (if (`self.canAttack`)
            (switch `int` (`self.CurrentAttack`)
              (:`Default`
                (if (<= (`KismetMathLibrary.Vector_Distance` (`self.K2_GetActorLocation`) (`self.K2_GetActorLocation` (`GameplayStatics.GetPlayerCharacter` 0))) (`self.PunchDistance`)) :!label _label
                  (set `self.canAttack` false)
                  (`CharacterMovementComponent.DisableMovement` (`self.CharacterMovement`))
                  (`KismetSystemLibrary.Delay` 0.5)
                  (`SkeletalMeshComponent.PlayAnimation` (`self.Mesh`) "/Game/Assets/3D/Boss/mutant_punch.mutant_punch" false)
                  (`KismetSystemLibrary.Delay` 0.25)
                  ;[1 1 1] Applying Damage
                  (bind _outactors (`KismetSystemLibrary.SphereOverlapActors` (`SceneComponent.K2_GetComponentLocation` (`self.Punch`)) 50.0 (`self.Object Types`)))
                  (for _array_element _outactors
                    (if (`self.ActorHasTag` _array_element "Player")
                      (`GameplayStatics.ApplyDamage` _array_element 5.0)))
                  (`KismetSystemLibrary.Delay` 0.75)
                  (`CharacterMovementComponent.SetMovementMode` (`self.CharacterMovement`) "MOVE_Walking" 0)
                  (`SkeletalMeshComponent.SetAnimationMode` _mesh "AnimationBlueprint")
                  (`SkeletalMeshComponent.SetAnimInstanceClass` _mesh "/Game/Animations/ABP_Boss.ABP_Boss_C")
                  (set `self.canAttack` true)
                  (switch `int` (`KismetMathLibrary.RandomInteger` 2)
                    (:`0`
                      (set `self.CurrentAttack` 0))
                    (:`1`
                      (set `self.CurrentAttack` 1)))))
              (:`0`
                (goto _label))
              (:`1`
                (if (<= (`KismetMathLibrary.Vector_Distance` (`self.K2_GetActorLocation`) (`self.K2_GetActorLocation` (`GameplayStatics.GetPlayerCharacter` 0))) (`self.JumpReachDistance`))
                  (set `self.canAttack` false)
                  (`CharacterMovementComponent.DisableMovement` (`self.CharacterMovement`))
                  (`SkeletalMeshComponent.PlayAnimation` (`self.Mesh`) "/Game/Assets/3D/Boss/mutent_prepare_slam.mutent_prepare_slam" false)
                  (`KismetSystemLibrary.Delay` 1.5)
                  (`KismetSystemLibrary.Delay` 0.25)
                  (set `self.JumpMove` (+ (* (* (`KismetMathLibrary.Normal` (- (`self.K2_GetActorLocation` (`GameplayStatics.GetPlayerCharacter` 0)) _returnvalue)) (`self.JumpDistance`)) (1.0 1.0 0.0)) _returnvalue))
                  (bind _outactors_2 (`KismetSystemLibrary.SphereOverlapActors` (`SceneComponent.K2_GetComponentLocation` (`self.Slam`)) 180.0 (`self.Object Types`)))
                  (for _array_element_2 _outactors_2
                    (if (`self.ActorHasTag` _array_element_2 "Player")
                      (`GameplayStatics.ApplyDamage` _array_element_2 7.5)))
                  (`KismetSystemLibrary.Delay` 1.0)
                  (`self.K2_SetActorLocation` (`self.JumpMove`))
                  (`CharacterMovementComponent.SetMovementMode` (`self.CharacterMovement`) "MOVE_Walking" 0)
                  (`SkeletalMeshComponent.SetAnimationMode` _mesh_2 "AnimationBlueprint")
                  (`SkeletalMeshComponent.SetAnimInstanceClass` _mesh_2 "/Game/Animations/ABP_Boss.ABP_Boss_C")
                  (set `self.canAttack` true)
                  (switch `int` (`KismetMathLibrary.RandomInteger` 2)
                    (:`0`
                      (set `self.CurrentAttack` 0))
                    (:`1`
                      (set `self.CurrentAttack` 1))))))))))))

(event `self.ReceiveAnyDamage`
  (params (Damage :type "Float (single-precision)") (DamageType :type "DamageType Object Reference") (InstigatedBy :type "Controller Object Reference") (DamageCauser :type "Actor Object Reference"))
  (bind _returnvalue (+ (`self.K2_GetActorLocation`) (-500.0 0.0 0.0)))
  ;[1 1 1] On Hit events
  (`|ExecutionSequence`
    (:`then_0`
      ;[1 1 1] Health System
      (set `self.Health` (- (`self.Health`) Damage))
      (`KismetSystemLibrary.PrintString` (`KismetStringLibrary.Conv_DoubleToString` (`self.Health`)))
      (if (<= (`self.Health`) 0.0)
        (`self.K2_DestroyActor`)
        (`KismetSystemLibrary.PrintString` "U has win")))
    (:`then_1`
      ;[1 1 1] Healing Blood
      (bind _result (`/Engine/EditorBlueprintResources/StandardMacros.IncrementInt` (`self.Blood spawn`))
        (:`  `
          (bind _output_get (set `self.Blood spawn` _result))
          (`KismetSystemLibrary.PrintString` (`KismetStringLibrary.Conv_IntToString` _output_get))
          (if (== (mod (`self.Blood spawn`) 3) 1)
            ;;[1 1 1] Spawning behind enemy
            (bind _outhit (`KismetSystemLibrary.LineTraceSingleForObjects` _returnvalue (+ _returnvalue (0.0 0.0 -200.0)) (`|MakeArray` (enumliteral `EObjectTypeQuery` "ObjectTypeQuery1"))))
            (`|SpawnActorFromClass` "/Game/HealingBlood.HealingBlood_C" (`KismetMathLibrary.Conv_VectorToTransform` (+ (`.Location` (`GameplayStatics.BreakHitResult` _outhit)) (5.0 0.0 7.0))) "AdjustIfPossibleButAlwaysSpawn" "OverrideRootScale" null null)
            (`KismetSystemLibrary.PrintString` "Spawned Blood")))))))

(fn `UserConstructionScript`)